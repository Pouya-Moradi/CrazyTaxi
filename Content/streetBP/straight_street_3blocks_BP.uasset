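; Straight street Blueprint, apparently a three-lane segment, that hands its spline paths to cars that enter it.
; Each of three box triggers reacts to overlapping Base_Car actors by copying the three splines into the car's Paths array.
; The box that was hit also sets ActivePathIndex to its matching spline, so the car's active path corresponds to its entry point.
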(event OnComponentBeginOverlap(Box0)
  (params (OverlappedComponent :type Primitive%20Component%20Object%20Reference) (OtherActor :type Actor%20Object%20Reference) (OtherComp :type Primitive%20Component%20Object%20Reference) (OtherBodyIndex :type Integer) (bFromSweep :type Boolean) (SweepResult :type Hit%20Result%20Structure%20%28by%20ref%29))
  (bind _asbase_car (Utilities|Casting|CastToBase_Car OtherActor))
  (Variables|/Game/PolygonCity/Maps/Vehicle_BP/Base_Car_BP/Base_Car.Base_Car_C|SetPaths _asbase_car (Utilities|Array|MakeArray (Variables|Default|GetSpline%200) (Variables|Default|GetSpline%201) (Variables|Default|GetSpline%202)))
  (Variables|/Game/PolygonCity/Maps/Vehicle_BP/Base_Car_BP/Base_Car.Base_Car_C|SetActivePathIndex _asbase_car 0))

(event OnComponentBeginOverlap(Box1)
  (params (OverlappedComponent :type Primitive%20Component%20Object%20Reference) (OtherActor :type Actor%20Object%20Reference) (OtherComp :type Primitive%20Component%20Object%20Reference) (OtherBodyIndex :type Integer) (bFromSweep :type Boolean) (SweepResult :type Hit%20Result%20Structure%20%28by%20ref%29))
  (bind _asbase_car (Utilities|Casting|CastToBase_Car OtherActor))
  (Variables|/Game/PolygonCity/Maps/Vehicle_BP/Base_Car_BP/Base_Car.Base_Car_C|SetPaths _asbase_car (Utilities|Array|MakeArray (Variables|Default|GetSpline%200) (Variables|Default|GetSpline%201) (Variables|Default|GetSpline%202)))
  (Variables|/Game/PolygonCity/Maps/Vehicle_BP/Base_Car_BP/Base_Car.Base_Car_C|SetActivePathIndex _asbase_car 1))

(event OnComponentBeginOverlap(Box2)
  (params (OverlappedComponent :type Primitive%20Component%20Object%20Reference) (OtherActor :type Actor%20Object%20Reference) (OtherComp :type Primitive%20Component%20Object%20Reference) (OtherBodyIndex :type Integer) (bFromSweep :type Boolean) (SweepResult :type Hit%20Result%20Structure%20%28by%20ref%29))
  (bind _asbase_car (Utilities|Casting|CastToBase_Car OtherActor))
  (Variables|/Game/PolygonCity/Maps/Vehicle_BP/Base_Car_BP/Base_Car.Base_Car_C|SetPaths _asbase_car (Utilities|Array|MakeArray (Variables|Default|GetSpline%200) (Variables|Default|GetSpline%201) (Variables|Default|GetSpline%202)))
  (Variables|/Game/PolygonCity/Maps/Vehicle_BP/Base_Car_BP/Base_Car.Base_Car_C|SetActivePathIndex _asbase_car 2))

(fn ConstructionScript)