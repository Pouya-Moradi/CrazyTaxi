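; Traffic light actor that stops and releases Base_Car vehicles through a Box trigger.
; BeginPlay waits an initial offset, then toggles IsRed in an endless Delay loop with separate red and green durations.
; Cars entering the box on red save their state, are flagged as behind the light and go idle, unless in the first enum state.
; Turning green restores each overlapping car's previous state.
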(event OnComponentBeginOverlap(Box)
  (params (OverlappedComponent :type Primitive%20Component%20Object%20Reference) (OtherActor :type Actor%20Object%20Reference) (OtherComp :type Primitive%20Component%20Object%20Reference) (OtherBodyIndex :type Integer) (bFromSweep :type Boolean) (SweepResult :type Hit%20Result%20Structure%20%28by%20ref%29))
  (if (Variables|Default|GetIsRed)
    (bind _asbase_car (Utilities|Casting|CastToBase_Car OtherActor))
    (if (Utilities|Enum|NotEqual(Enum) (Variables|/Game/PolygonCity/Maps/BluePrints/Base_Car_BP/Base_Car.Base_Car_C|GetState _asbase_car) "NewEnumerator0")
      (Variables|/Game/PolygonCity/Maps/BluePrints/Base_Car_BP/Base_Car.Base_Car_C|SetPreviousState _asbase_car (Variables|/Game/PolygonCity/Maps/BluePrints/Base_Car_BP/Base_Car.Base_Car_C|GetState _asbase_car))
      (Variables|/Game/PolygonCity/Maps/BluePrints/Base_Car_BP/Base_Car.Base_Car_C|SetIsBehindTrafficLight _asbase_car true)
      (Default|GotoIdling _asbase_car))))

(event EventBeginPlay
  (Utilities|FlowControl|Delay (Variables|Default|GetInitialDelay))
  (if (Variables|Default|GetIsRed) :!label _label
    (Utilities|FlowControl|Delay (Variables|Default|GetRedTime))
    (Variables|Default|SetIsRed false)
    (Utilities|FlowControl|Sequence
      (:then_0
        (goto _label))
      (:then_1
        (for _array_element (Collision|GetOverlappingActors (Variables|Default|GetBox) "/Game/PolygonCity/Maps/BluePrints/Base_Car_BP/Base_Car.Base_Car_C" :!class /Script/Engine.PrimitiveComponent)
          (bind _asbase_car (Utilities|Casting|CastToBase_Car _array_element))
          (Default|GotoStatewithPreviousData _asbase_car (Variables|/Game/PolygonCity/Maps/BluePrints/Base_Car_BP/Base_Car.Base_Car_C|GetPreviousState _asbase_car)))))
    (else
      (Utilities|FlowControl|Delay (Variables|Default|GetGreenTime))
      (Variables|Default|SetIsRed true)
      (goto _label))))

(fn ConstructionScript)