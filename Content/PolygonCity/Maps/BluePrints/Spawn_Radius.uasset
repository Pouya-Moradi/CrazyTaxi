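; Spawn_Radius is an actor that regulates car density inside its Sphere component.
; From one second after BeginPlay, it repeats a check every second, counting overlapping Base_Car actors against Population.
; While the count does not exceed Population, it calls CheckDensity on each overlapping three-, two- and one-line Blueprint actor, leaving the density response to those actors.
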(event EventBeginPlay
  (bind _sphere (Variables|Default|GetSphere))
  (Utilities|FlowControl|Delay 1.0)
  (if (> (Utilities|Array|Length (Collision|GetOverlappingActors _sphere "/Game/PolygonCity/Maps/BluePrints/Base_Car_BP/Base_Car.Base_Car_C" :!class /Script/Engine.PrimitiveComponent)) (Variables|Default|GetPopulation)) :!label _label
    _
    (else
      (for _array_element (Collision|GetOverlappingActors _sphere "/Game/PolygonCity/Maps/BluePrints/Base_Car_BP/street_BP/three_line_BP.three_line_BP_C" :!class /Script/Engine.PrimitiveComponent)
        (bind _asthree_line_bp (Utilities|Casting|CastTothree_line_BP _array_element))
        (Default|CheckDensity _asthree_line_bp))
      (for _array_element_2 (Collision|GetOverlappingActors _sphere "/Game/PolygonCity/Maps/BluePrints/Base_Car_BP/street_BP/two_line_BP.two_line_BP_C" :!class /Script/Engine.PrimitiveComponent)
        (bind _astwo_line_bp (Utilities|Casting|CastTotwo_line_BP _array_element_2))
        (Default|CheckDensity _astwo_line_bp))
      (for _array_element_3 (Collision|GetOverlappingActors _sphere "/Game/PolygonCity/Maps/BluePrints/Base_Car_BP/street_BP/one_line_BP.one_line_BP_C" :!class /Script/Engine.PrimitiveComponent)
        (bind _asone_line_bp (Utilities|Casting|CastToone_line_BP _array_element_3))
        (Default|CheckDensity _asone_line_bp))))
  (Utilities|FlowControl|Delay 1.0)
  (goto _label))

(fn ConstructionScript)