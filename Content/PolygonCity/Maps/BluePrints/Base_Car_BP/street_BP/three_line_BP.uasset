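; Three-lane street segment that feeds lane splines, a speed limit and a GUID to Base_Car vehicles entering it.
; Each lane's collision volume sets the car's active path, with IsParkable dropping the first lane from the drivable paths.
; CheckDensity spawns a random AI car when the Density volume holds two or fewer.
; Six spawn points map in pairs to lanes, and parkable streets skip the first pair.
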(event OnComponentBeginOverlap(collision0)
  (params (OverlappedComponent :type Primitive%20Component%20Object%20Reference) (OtherActor :type Actor%20Object%20Reference) (OtherComp :type Primitive%20Component%20Object%20Reference) (OtherBodyIndex :type Integer) (bFromSweep :type Boolean) (SweepResult :type Hit%20Result%20Structure%20%28by%20ref%29))
  (bind _spline_2 (Variables|Default|GetSpline%202))
  (bind _spline_1 (Variables|Default|GetSpline%201))
  (bind _asbase_car (Utilities|Casting|CastToBase_Car OtherActor))
  (if (Variables|Default|GetIsParkable)
    (Variables|/Game/PolygonCity/Maps/BluePrints/Base_Car_BP/Base_Car.Base_Car_C|SetPaths _asbase_car (Utilities|Array|MakeArray _spline_1 _spline_2))
    (else
      (Variables|/Game/PolygonCity/Maps/BluePrints/Base_Car_BP/Base_Car.Base_Car_C|SetPaths _asbase_car (Utilities|Array|MakeArray (Variables|Default|GetSpline%200) _spline_1 _spline_2))))
  (Variables|/Game/PolygonCity/Maps/BluePrints/Base_Car_BP/Base_Car.Base_Car_C|SetActivePathIndex _asbase_car 0)
  (Variables|/Game/PolygonCity/Maps/BluePrints/Base_Car_BP/Base_Car.Base_Car_C|SetStreetSpeedLimit _asbase_car (Variables|Default|GetSpeedLimit))
  (Variables|/Game/PolygonCity/Maps/BluePrints/Base_Car_BP/Base_Car.Base_Car_C|SetStreetGUID _asbase_car (Variables|Default|GetGUID)))

(event OnComponentBeginOverlap(collision1)
  (params (OverlappedComponent :type Primitive%20Component%20Object%20Reference) (OtherActor :type Actor%20Object%20Reference) (OtherComp :type Primitive%20Component%20Object%20Reference) (OtherBodyIndex :type Integer) (bFromSweep :type Boolean) (SweepResult :type Hit%20Result%20Structure%20%28by%20ref%29))
  (bind _spline_2 (Variables|Default|GetSpline%202))
  (bind _spline_1 (Variables|Default|GetSpline%201))
  (bind _asbase_car (Utilities|Casting|CastToBase_Car OtherActor))
  (if (Variables|Default|GetIsParkable)
    (Variables|/Game/PolygonCity/Maps/BluePrints/Base_Car_BP/Base_Car.Base_Car_C|SetPaths _asbase_car (Utilities|Array|MakeArray _spline_1 _spline_2))
    (Variables|/Game/PolygonCity/Maps/BluePrints/Base_Car_BP/Base_Car.Base_Car_C|SetActivePathIndex _asbase_car 0)
    (else
      (Variables|/Game/PolygonCity/Maps/BluePrints/Base_Car_BP/Base_Car.Base_Car_C|SetPaths _asbase_car (Utilities|Array|MakeArray (Variables|Default|GetSpline%200) _spline_1 _spline_2))
      (Variables|/Game/PolygonCity/Maps/BluePrints/Base_Car_BP/Base_Car.Base_Car_C|SetActivePathIndex _asbase_car 1)))
  (Variables|/Game/PolygonCity/Maps/BluePrints/Base_Car_BP/Base_Car.Base_Car_C|SetStreetSpeedLimit _asbase_car (Variables|Default|GetSpeedLimit))
  (Variables|/Game/PolygonCity/Maps/BluePrints/Base_Car_BP/Base_Car.Base_Car_C|SetStreetGUID _asbase_car (Variables|Default|GetGUID)))

(event OnComponentBeginOverlap(collision2)
  (params (OverlappedComponent :type Primitive%20Component%20Object%20Reference) (OtherActor :type Actor%20Object%20Reference) (OtherComp :type Primitive%20Component%20Object%20Reference) (OtherBodyIndex :type Integer) (bFromSweep :type Boolean) (SweepResult :type Hit%20Result%20Structure%20%28by%20ref%29))
  (bind _spline_2 (Variables|Default|GetSpline%202))
  (bind _spline_1 (Variables|Default|GetSpline%201))
  (bind _asbase_car (Utilities|Casting|CastToBase_Car OtherActor))
  (if (Variables|Default|GetIsParkable)
    (Variables|/Game/PolygonCity/Maps/BluePrints/Base_Car_BP/Base_Car.Base_Car_C|SetPaths _asbase_car (Utilities|Array|MakeArray _spline_1 _spline_2))
    (Variables|/Game/PolygonCity/Maps/BluePrints/Base_Car_BP/Base_Car.Base_Car_C|SetActivePathIndex _asbase_car 1)
    (else
      (Variables|/Game/PolygonCity/Maps/BluePrints/Base_Car_BP/Base_Car.Base_Car_C|SetPaths _asbase_car (Utilities|Array|MakeArray (Variables|Default|GetSpline%200) _spline_1 _spline_2))
      (Variables|/Game/PolygonCity/Maps/BluePrints/Base_Car_BP/Base_Car.Base_Car_C|SetActivePathIndex _asbase_car 2)))
  (Variables|/Game/PolygonCity/Maps/BluePrints/Base_Car_BP/Base_Car.Base_Car_C|SetStreetSpeedLimit _asbase_car (Variables|Default|GetSpeedLimit))
  (Variables|/Game/PolygonCity/Maps/BluePrints/Base_Car_BP/Base_Car.Base_Car_C|SetStreetGUID _asbase_car (Variables|Default|GetGUID)))

(event EventBeginPlay
  (Utilities|Struct|SetmembersinGuid (Guid|NewGuid)))

(fn ConstructionScript)

(fn CheckDensity
  (bind _density (Variables|Default|GetDensity))
  (bind _overlappingactors (Collision|GetOverlappingActors _density "/Game/PolygonCity/Maps/BluePrints/Base_Car_BP/Base_Car.Base_Car_C" :!class /Script/Engine.PrimitiveComponent))
  (bind _returnvalue (Utilities|Array|Length _overlappingactors))
  (bind _returnvalue_2 (> _returnvalue 2))
  (if (Variables|Default|GetIsParkable)
    (if (not _returnvalue_2)
      (CallFunction|Spawn (Math|Random|RandomIntegerinRange 2 5)))
    (elif (not _returnvalue_2)
      (CallFunction|Spawn (Math|Random|RandomIntegerinRange 0 5)))))

(fn Spawn
  (params (Index :type Integer))
  (bind _returnvalue (/ Index 2))
  (bind _cars (Variables|Default|GetCars))
  (bind _spawn_point_0 (Variables|Default|GetSpawn%20Point%200))
  (bind _spawn_point_5 (Variables|Default|GetSpawn%20Point%205))
  (bind _spawn_point_3 (Variables|Default|GetSpawn%20Point%203))
  (bind _spawn_point_4 (Variables|Default|GetSpawn%20Point%204))
  (bind _spawn_point_1 (Variables|Default|GetSpawn%20Point%201))
  (bind _spawn_point_2 (Variables|Default|GetSpawn%20Point%202))
  (bind _spline_2 (Variables|Default|GetSpline%202))
  (bind _spline_1 (Variables|Default|GetSpline%201))
  (bind _array (Utilities|Array|MakeArray _spawn_point_0 _spawn_point_1 _spawn_point_2 _spawn_point_3 _spawn_point_4 _spawn_point_5))
  (bind _output (Utilities|Array|Get(acopy) _array Index))
  (bind _returnvalue_2 (AI|SpawnAIFromClass (Utilities|Array|Get(acopy) _cars (Math|Random|RandomInteger (Utilities|Array|Length _cars))) 0 (Transformation|GetWorldLocation _output) (Transformation|GetWorldRotation _output) false 0))
  (bind _asbase_car (Utilities|Casting|CastToBase_Car _returnvalue_2))
  (if (Variables|Default|GetIsParkable)
    (Variables|/Game/PolygonCity/Maps/BluePrints/Base_Car_BP/Base_Car.Base_Car_C|SetActivePathIndex _asbase_car (- _returnvalue 1))
    (Variables|/Game/PolygonCity/Maps/BluePrints/Base_Car_BP/Base_Car.Base_Car_C|SetPaths _asbase_car (Utilities|Array|MakeArray _spline_1 _spline_2))
    (else
      (Variables|/Game/PolygonCity/Maps/BluePrints/Base_Car_BP/Base_Car.Base_Car_C|SetActivePathIndex _asbase_car _returnvalue)
      (Variables|/Game/PolygonCity/Maps/BluePrints/Base_Car_BP/Base_Car.Base_Car_C|SetPaths _asbase_car (Utilities|Array|MakeArray (Variables|Default|GetSpline%200) _spline_1 _spline_2))))
  (Variables|/Game/PolygonCity/Maps/BluePrints/Base_Car_BP/Base_Car.Base_Car_C|SetStreetSpeedLimit _asbase_car (Variables|Default|GetSpeedLimit))
  (Variables|/Game/PolygonCity/Maps/BluePrints/Base_Car_BP/Base_Car.Base_Car_C|SetState _asbase_car "NewEnumerator3")
  (Default|InitializeAIState _asbase_car))