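; One-lane street Blueprint that routes AI traffic cars along a single spline.
; On BeginPlay it creates a GUID, and cars entering its collision volume receive the spline, speed limit and that GUID.
; CheckDensity spawns a random car at one of two spawn points unless over two cars overlap the Density component.
; Spawned cars get the spline, speed limit and a state before their AI initializes.
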(event OnComponentBeginOverlap(collision0)
  (params (OverlappedComponent :type Primitive%20Component%20Object%20Reference) (OtherActor :type Actor%20Object%20Reference) (OtherComp :type Primitive%20Component%20Object%20Reference) (OtherBodyIndex :type Integer) (bFromSweep :type Boolean) (SweepResult :type Hit%20Result%20Structure%20%28by%20ref%29))
  (bind _asbase_car (Utilities|Casting|CastToBase_Car OtherActor))
  (Variables|/Game/PolygonCity/Maps/BluePrints/Base_Car_BP/Base_Car.Base_Car_C|SetPaths _asbase_car (Utilities|Array|MakeArray (Variables|Default|GetSpline%200)))
  (Variables|/Game/PolygonCity/Maps/BluePrints/Base_Car_BP/Base_Car.Base_Car_C|SetActivePathIndex _asbase_car 0)
  (Variables|/Game/PolygonCity/Maps/BluePrints/Base_Car_BP/Base_Car.Base_Car_C|SetStreetSpeedLimit _asbase_car (Variables|Default|GetSpeedLimit))
  (Variables|/Game/PolygonCity/Maps/BluePrints/Base_Car_BP/Base_Car.Base_Car_C|SetStreetGUID _asbase_car (Variables|Default|GetGUID)))

(event EventBeginPlay
  (Utilities|Struct|SetmembersinGuid (Guid|NewGuid)))

(fn ConstructionScript)

(fn CheckDensity
  (if (not (> (Utilities|Array|Length (Collision|GetOverlappingActors (Variables|Default|GetDensity) "/Game/PolygonCity/Maps/BluePrints/Base_Car_BP/Base_Car.Base_Car_C" :!class /Script/Engine.PrimitiveComponent)) 2))
    (CallFunction|Spawn (Math|Random|RandomIntegerinRange 0 1))))

(fn Spawn
  (params (Index :type Integer))
  (bind _cars (Variables|Default|GetCars))
  (bind _spawn_point_0 (Variables|Default|GetSpawn%20Point%200))
  (bind _spawn_point_1 (Variables|Default|GetSpawn%20Point%201))
  (bind _array (Utilities|Array|MakeArray _spawn_point_0 _spawn_point_1))
  (bind _output (Utilities|Array|Get(acopy) _array Index))
  (bind _returnvalue (AI|SpawnAIFromClass (Utilities|Array|Get(acopy) _cars (Math|Random|RandomInteger (Utilities|Array|Length _cars))) 0 (Transformation|GetWorldLocation _output) (Transformation|GetWorldRotation _output) false 0))
  (bind _asbase_car (Utilities|Casting|CastToBase_Car _returnvalue))
  (Variables|/Game/PolygonCity/Maps/BluePrints/Base_Car_BP/Base_Car.Base_Car_C|SetActivePathIndex _asbase_car (/ Index 2))
  (Variables|/Game/PolygonCity/Maps/BluePrints/Base_Car_BP/Base_Car.Base_Car_C|SetPaths _asbase_car (Utilities|Array|MakeArray (Variables|Default|GetSpline%200)))
  (Variables|/Game/PolygonCity/Maps/BluePrints/Base_Car_BP/Base_Car.Base_Car_C|SetStreetSpeedLimit _asbase_car (Variables|Default|GetSpeedLimit))
  (Variables|/Game/PolygonCity/Maps/BluePrints/Base_Car_BP/Base_Car.Base_Car_C|SetState _asbase_car "NewEnumerator3")
  (Default|InitializeAIState _asbase_car))