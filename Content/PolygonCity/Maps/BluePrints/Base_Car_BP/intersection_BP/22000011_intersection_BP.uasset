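; Intersection Blueprint that routes Base_Car vehicles through a junction using trigger boxes and spline paths.
; When a car in one specific State overlaps one of three boxes, its Paths array is replaced with that box's spline and its active path index resets to the start.
; Box feeds Spline6, while Box9 and Box11 both feed Spline3.
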(event OnComponentBeginOverlap(Box9)
  (params (OverlappedComponent :type Primitive%20Component%20Object%20Reference) (OtherActor :type Actor%20Object%20Reference) (OtherComp :type Primitive%20Component%20Object%20Reference) (OtherBodyIndex :type Integer) (bFromSweep :type Boolean) (SweepResult :type Hit%20Result%20Structure%20%28by%20ref%29))
  (bind _asbase_car (Utilities|Casting|CastToBase_Car OtherActor))
  (if (Utilities|Enum|Equal(Enum) (Variables|/Game/PolygonCity/Maps/BluePrints/Base_Car_BP/Base_Car.Base_Car_C|GetState _asbase_car) "NewEnumerator3")
    (Variables|/Game/PolygonCity/Maps/BluePrints/Base_Car_BP/Base_Car.Base_Car_C|SetPaths _asbase_car (Utilities|Array|MakeArray (Variables|Default|GetSpline3)))
    (Variables|/Game/PolygonCity/Maps/BluePrints/Base_Car_BP/Base_Car.Base_Car_C|SetActivePathIndex _asbase_car 0)))

(event OnComponentBeginOverlap(Box11)
  (params (OverlappedComponent :type Primitive%20Component%20Object%20Reference) (OtherActor :type Actor%20Object%20Reference) (OtherComp :type Primitive%20Component%20Object%20Reference) (OtherBodyIndex :type Integer) (bFromSweep :type Boolean) (SweepResult :type Hit%20Result%20Structure%20%28by%20ref%29))
  (bind _asbase_car (Utilities|Casting|CastToBase_Car OtherActor))
  (if (Utilities|Enum|Equal(Enum) (Variables|/Game/PolygonCity/Maps/BluePrints/Base_Car_BP/Base_Car.Base_Car_C|GetState _asbase_car) "NewEnumerator3")
    (Variables|/Game/PolygonCity/Maps/BluePrints/Base_Car_BP/Base_Car.Base_Car_C|SetPaths _asbase_car (Utilities|Array|MakeArray (Variables|Default|GetSpline3)))
    (Variables|/Game/PolygonCity/Maps/BluePrints/Base_Car_BP/Base_Car.Base_Car_C|SetActivePathIndex _asbase_car 0)))

(event OnComponentBeginOverlap(Box)
  (params (OverlappedComponent :type Primitive%20Component%20Object%20Reference) (OtherActor :type Actor%20Object%20Reference) (OtherComp :type Primitive%20Component%20Object%20Reference) (OtherBodyIndex :type Integer) (bFromSweep :type Boolean) (SweepResult :type Hit%20Result%20Structure%20%28by%20ref%29))
  (bind _asbase_car (Utilities|Casting|CastToBase_Car OtherActor))
  (if (Utilities|Enum|Equal(Enum) (Variables|/Game/PolygonCity/Maps/BluePrints/Base_Car_BP/Base_Car.Base_Car_C|GetState _asbase_car) "NewEnumerator3")
    (Variables|/Game/PolygonCity/Maps/BluePrints/Base_Car_BP/Base_Car.Base_Car_C|SetPaths _asbase_car (Utilities|Array|MakeArray (Variables|Default|GetSpline6)))
    (Variables|/Game/PolygonCity/Maps/BluePrints/Base_Car_BP/Base_Car.Base_Car_C|SetActivePathIndex _asbase_car 0)))

(fn ConstructionScript)