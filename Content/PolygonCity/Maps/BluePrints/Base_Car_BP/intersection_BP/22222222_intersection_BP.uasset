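; Road intersection actor that routes Base_Car vehicles onto randomly chosen spline paths as they enter it.
; Eight trigger boxes, in pairs sharing four candidate splines, act only on cars in one specific State enum value.
; On overlap, a box replaces the car's Paths with one random spline and resets ActivePathIndex to zero.
; Box10 and Box11 roll six values over four splines, so their index can fall out of range.
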(event OnComponentBeginOverlap(Box10)
  (params (OverlappedComponent :type Primitive%20Component%20Object%20Reference) (OtherActor :type Actor%20Object%20Reference) (OtherComp :type Primitive%20Component%20Object%20Reference) (OtherBodyIndex :type Integer) (bFromSweep :type Boolean) (SweepResult :type Hit%20Result%20Structure%20%28by%20ref%29))
  (bind _asbase_car (Utilities|Casting|CastToBase_Car OtherActor))
  (if (Utilities|Enum|Equal(Enum) (Variables|/Game/PolygonCity/Maps/BluePrints/Base_Car_BP/Base_Car.Base_Car_C|GetState _asbase_car) "NewEnumerator3")
    (Variables|/Game/PolygonCity/Maps/BluePrints/Base_Car_BP/Base_Car.Base_Car_C|SetPaths _asbase_car (Utilities|Array|MakeArray (Utilities|Array|Get(acopy) (Utilities|Array|MakeArray (Variables|Default|GetSpline11) (Variables|Default|GetSpline10) (Variables|Default|GetSpline4) (Variables|Default|GetSpline3)) (Math|Random|RandomInteger 6))))
    (Variables|/Game/PolygonCity/Maps/BluePrints/Base_Car_BP/Base_Car.Base_Car_C|SetActivePathIndex _asbase_car 0)))

(event OnComponentBeginOverlap(Box1)
  (params (OverlappedComponent :type Primitive%20Component%20Object%20Reference) (OtherActor :type Actor%20Object%20Reference) (OtherComp :type Primitive%20Component%20Object%20Reference) (OtherBodyIndex :type Integer) (bFromSweep :type Boolean) (SweepResult :type Hit%20Result%20Structure%20%28by%20ref%29))
  (bind _asbase_car (Utilities|Casting|CastToBase_Car OtherActor))
  (if (Utilities|Enum|Equal(Enum) (Variables|/Game/PolygonCity/Maps/BluePrints/Base_Car_BP/Base_Car.Base_Car_C|GetState _asbase_car) "NewEnumerator3")
    (Variables|/Game/PolygonCity/Maps/BluePrints/Base_Car_BP/Base_Car.Base_Car_C|SetPaths _asbase_car (Utilities|Array|MakeArray (Utilities|Array|Get(acopy) (Utilities|Array|MakeArray (Variables|Default|GetSpline7) (Variables|Default|GetSpline6) (Variables|Default|GetSpline2) (Variables|Default|GetSpline1)) (Math|Random|RandomInteger 4))))
    (Variables|/Game/PolygonCity/Maps/BluePrints/Base_Car_BP/Base_Car.Base_Car_C|SetActivePathIndex _asbase_car 0)))

(event OnComponentBeginOverlap(Box2)
  (params (OverlappedComponent :type Primitive%20Component%20Object%20Reference) (OtherActor :type Actor%20Object%20Reference) (OtherComp :type Primitive%20Component%20Object%20Reference) (OtherBodyIndex :type Integer) (bFromSweep :type Boolean) (SweepResult :type Hit%20Result%20Structure%20%28by%20ref%29))
  (bind _asbase_car (Utilities|Casting|CastToBase_Car OtherActor))
  (if (Utilities|Enum|Equal(Enum) (Variables|/Game/PolygonCity/Maps/BluePrints/Base_Car_BP/Base_Car.Base_Car_C|GetState _asbase_car) "NewEnumerator3")
    (Variables|/Game/PolygonCity/Maps/BluePrints/Base_Car_BP/Base_Car.Base_Car_C|SetPaths _asbase_car (Utilities|Array|MakeArray (Utilities|Array|Get(acopy) (Utilities|Array|MakeArray (Variables|Default|GetSpline7) (Variables|Default|GetSpline6) (Variables|Default|GetSpline2) (Variables|Default|GetSpline1)) (Math|Random|RandomInteger 4))))
    (Variables|/Game/PolygonCity/Maps/BluePrints/Base_Car_BP/Base_Car.Base_Car_C|SetActivePathIndex _asbase_car 0)))

(event OnComponentBeginOverlap(Box11)
  (params (OverlappedComponent :type Primitive%20Component%20Object%20Reference) (OtherActor :type Actor%20Object%20Reference) (OtherComp :type Primitive%20Component%20Object%20Reference) (OtherBodyIndex :type Integer) (bFromSweep :type Boolean) (SweepResult :type Hit%20Result%20Structure%20%28by%20ref%29))
  (bind _asbase_car (Utilities|Casting|CastToBase_Car OtherActor))
  (if (Utilities|Enum|Equal(Enum) (Variables|/Game/PolygonCity/Maps/BluePrints/Base_Car_BP/Base_Car.Base_Car_C|GetState _asbase_car) "NewEnumerator3")
    (Variables|/Game/PolygonCity/Maps/BluePrints/Base_Car_BP/Base_Car.Base_Car_C|SetPaths _asbase_car (Utilities|Array|MakeArray (Utilities|Array|Get(acopy) (Utilities|Array|MakeArray (Variables|Default|GetSpline11) (Variables|Default|GetSpline10) (Variables|Default|GetSpline4) (Variables|Default|GetSpline3)) (Math|Random|RandomInteger 6))))
    (Variables|/Game/PolygonCity/Maps/BluePrints/Base_Car_BP/Base_Car.Base_Car_C|SetActivePathIndex _asbase_car 0)))

(event OnComponentBeginOverlap(Box7)
  (params (OverlappedComponent :type Primitive%20Component%20Object%20Reference) (OtherActor :type Actor%20Object%20Reference) (OtherComp :type Primitive%20Component%20Object%20Reference) (OtherBodyIndex :type Integer) (bFromSweep :type Boolean) (SweepResult :type Hit%20Result%20Structure%20%28by%20ref%29))
  (bind _asbase_car (Utilities|Casting|CastToBase_Car OtherActor))
  (if (Utilities|Enum|Equal(Enum) (Variables|/Game/PolygonCity/Maps/BluePrints/Base_Car_BP/Base_Car.Base_Car_C|GetState _asbase_car) "NewEnumerator3")
    (Variables|/Game/PolygonCity/Maps/BluePrints/Base_Car_BP/Base_Car.Base_Car_C|SetPaths _asbase_car (Utilities|Array|MakeArray (Utilities|Array|Get(acopy) (Utilities|Array|MakeArray (Variables|Default|GetSpline7) (Variables|Default|GetSpline6) (Variables|Default|GetSpline4) (Variables|Default|GetSpline3)) (Math|Random|RandomInteger 4))))
    (Variables|/Game/PolygonCity/Maps/BluePrints/Base_Car_BP/Base_Car.Base_Car_C|SetActivePathIndex _asbase_car 0)))

(event OnComponentBeginOverlap(Box6)
  (params (OverlappedComponent :type Primitive%20Component%20Object%20Reference) (OtherActor :type Actor%20Object%20Reference) (OtherComp :type Primitive%20Component%20Object%20Reference) (OtherBodyIndex :type Integer) (bFromSweep :type Boolean) (SweepResult :type Hit%20Result%20Structure%20%28by%20ref%29))
  (bind _asbase_car (Utilities|Casting|CastToBase_Car OtherActor))
  (if (Utilities|Enum|Equal(Enum) (Variables|/Game/PolygonCity/Maps/BluePrints/Base_Car_BP/Base_Car.Base_Car_C|GetState _asbase_car) "NewEnumerator3")
    (Variables|/Game/PolygonCity/Maps/BluePrints/Base_Car_BP/Base_Car.Base_Car_C|SetPaths _asbase_car (Utilities|Array|MakeArray (Utilities|Array|Get(acopy) (Utilities|Array|MakeArray (Variables|Default|GetSpline7) (Variables|Default|GetSpline6) (Variables|Default|GetSpline4) (Variables|Default|GetSpline3)) (Math|Random|RandomInteger 4))))
    (Variables|/Game/PolygonCity/Maps/BluePrints/Base_Car_BP/Base_Car.Base_Car_C|SetActivePathIndex _asbase_car 0)))

(event OnComponentBeginOverlap(Box3)
  (params (OverlappedComponent :type Primitive%20Component%20Object%20Reference) (OtherActor :type Actor%20Object%20Reference) (OtherComp :type Primitive%20Component%20Object%20Reference) (OtherBodyIndex :type Integer) (bFromSweep :type Boolean) (SweepResult :type Hit%20Result%20Structure%20%28by%20ref%29))
  (bind _asbase_car (Utilities|Casting|CastToBase_Car OtherActor))
  (if (Utilities|Enum|Equal(Enum) (Variables|/Game/PolygonCity/Maps/BluePrints/Base_Car_BP/Base_Car.Base_Car_C|GetState _asbase_car) "NewEnumerator3")
    (Variables|/Game/PolygonCity/Maps/BluePrints/Base_Car_BP/Base_Car.Base_Car_C|SetPaths _asbase_car (Utilities|Array|MakeArray (Utilities|Array|Get(acopy) (Utilities|Array|MakeArray (Variables|Default|GetSpline4) (Variables|Default|GetSpline3) (Variables|Default|GetSpline11) (Variables|Default|GetSpline10)) (Math|Random|RandomInteger 4))))
    (Variables|/Game/PolygonCity/Maps/BluePrints/Base_Car_BP/Base_Car.Base_Car_C|SetActivePathIndex _asbase_car 0)))

(event OnComponentBeginOverlap(Box4)
  (params (OverlappedComponent :type Primitive%20Component%20Object%20Reference) (OtherActor :type Actor%20Object%20Reference) (OtherComp :type Primitive%20Component%20Object%20Reference) (OtherBodyIndex :type Integer) (bFromSweep :type Boolean) (SweepResult :type Hit%20Result%20Structure%20%28by%20ref%29))
  (bind _asbase_car (Utilities|Casting|CastToBase_Car OtherActor))
  (if (Utilities|Enum|Equal(Enum) (Variables|/Game/PolygonCity/Maps/BluePrints/Base_Car_BP/Base_Car.Base_Car_C|GetState _asbase_car) "NewEnumerator3")
    (Variables|/Game/PolygonCity/Maps/BluePrints/Base_Car_BP/Base_Car.Base_Car_C|SetPaths _asbase_car (Utilities|Array|MakeArray (Utilities|Array|Get(acopy) (Utilities|Array|MakeArray (Variables|Default|GetSpline4) (Variables|Default|GetSpline3) (Variables|Default|GetSpline11) (Variables|Default|GetSpline10)) (Math|Random|RandomInteger 4))))
    (Variables|/Game/PolygonCity/Maps/BluePrints/Base_Car_BP/Base_Car.Base_Car_C|SetActivePathIndex _asbase_car 0)))

(fn ConstructionScript)