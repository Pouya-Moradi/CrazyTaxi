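; Base AI traffic car driven by a state machine for random or targeted driving, parking, chasing a target car and idling.
; Tick updates the state and steers along spline paths or toward a target, while a looping cruise control adjusts throttle to the speed limit or chase speed.
; Trigger volumes stop it behind cars, switch lanes to overtake and propagate red-light status through queued cars.
; Stuck cars self-destroy once off screen.
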(event OnComponentBeginOverlap(StopTrigger)
  (params (OverlappedComponent :type Primitive%20Component%20Object%20Reference) (OtherActor :type Actor%20Object%20Reference) (OtherComp :type Primitive%20Component%20Object%20Reference) (OtherBodyIndex :type Integer) (bFromSweep :type Boolean) (SweepResult :type Hit%20Result%20Structure%20%28by%20ref%29))
  (bind _state (Variables|AI|GetState))
  ;[1 1 1] Avoid Cars
  (Utilities|Casting|CastToBase_Car OtherActor
    (:then
      _)
    (:CastFailed
      (Utilities|Casting|CastToBase_Car_BP OtherActor)))
  (if (Utilities|Enum|NotEqual(Enum) _state "NewEnumerator0")
    (Variables|AI|SetPreviousState _state)
    (CallFunction|GotoIdling)
    (Utilities|FlowControl|Delay 1e+01 :!label _label)
    (if (Utilities|Enum|Equal(Enum) _state "NewEnumerator0")
      (if (Variables|AI|GetIsBehindTrafficLight)
        (goto _label)
        (else
          (bind _isinview (CallFunction|IsinView :!label _label_2))
          (if _isinview
            (Utilities|FlowControl|Delay 0.1)
            (goto _label_2)
            (else
              (Actor|DestroyActor))))))))

(event OnComponentBeginOverlap(OvertakeTrigger)
  (params (OverlappedComponent :type Primitive%20Component%20Object%20Reference) (OtherActor :type Actor%20Object%20Reference) (OtherComp :type Primitive%20Component%20Object%20Reference) (OtherBodyIndex :type Integer) (bFromSweep :type Boolean) (SweepResult :type Hit%20Result%20Structure%20%28by%20ref%29))
  (bind _state (Variables|AI|GetState))
  ;[1 1 1] Overtake
  (bind _asbase_car (Utilities|Casting|CastToBase_Car OtherActor))
  (if (not (Variables|Base_Car_C|GetIsBehindTrafficLight _asbase_car))
    (if (== (Math|Random|RandomInteger (Variables|AI|GetOvertakeOdds)) 0)
      (if (Math|Boolean|ORBoolean (Utilities|Enum|Equal(Enum) _state "NewEnumerator6") (Utilities|Enum|Equal(Enum) _state "NewEnumerator5") (Utilities|Enum|Equal(Enum) _state "NewEnumerator4") (Utilities|Enum|Equal(Enum) _state "NewEnumerator3"))
        (if (> (Utilities|Array|Length (Variables|AI|GetPaths)) (+ (Variables|AI|GetActivePathIndex) 1))
          (if (== (Utilities|Array|Length (Collision|GetOverlappingActors (Variables|Default|GetOvertake%20Area%20Left) "Base_Car_C" :!class /Script/Engine.PrimitiveComponent)) 0)
            (Variables|AI|SetActivePathIndex (+ (Variables|AI|GetActivePathIndex) 1))
            (else
              (if (not (< (- (Variables|AI|GetActivePathIndex) 1) 0)) :!label _label
                (if (== (Utilities|Array|Length (Collision|GetOverlappingActors (Variables|Default|GetOvertake%20Area%20Right) "Base_Car_C" :!class /Script/Engine.PrimitiveComponent)) 0)
                  (Variables|AI|SetActivePathIndex (- (Variables|AI|GetActivePathIndex) 1))))))
          (else
            (goto _label)))))))

(event OnComponentEndOverlap(ClearZone)
  (params (OverlappedComponent :type Primitive%20Component%20Object%20Reference) (OtherActor :type Actor%20Object%20Reference) (OtherComp :type Primitive%20Component%20Object%20Reference) (OtherBodyIndex :type Integer))
  ;[1 1 1] Avoid Cars
  (Utilities|Casting|CastToBase_Car OtherActor
    (:then
      _)
    (:CastFailed
      (Utilities|Casting|CastToBase_Car_BP OtherActor)))
  (if (and (== (Utilities|Array|Length (Collision|GetOverlappingActors OverlappedComponent "Base_Car_C" :!class /Script/Engine.PrimitiveComponent)) 0) (== (Utilities|Array|Length (Collision|GetOverlappingActors OverlappedComponent "/Game/VehicleBP/Sedan/Base_Car_BP.Base_Car_BP_C" :!class /Script/Engine.PrimitiveComponent)) 0))
    (Variables|AI|SetIsBehindTrafficLight false)
    (CallFunction|GotoStatewithPreviousData (Variables|AI|GetPreviousState))))

(event OnComponentBeginOverlap(RedLightZone)
  (params (OverlappedComponent :type Primitive%20Component%20Object%20Reference) (OtherActor :type Actor%20Object%20Reference) (OtherComp :type Primitive%20Component%20Object%20Reference) (OtherBodyIndex :type Integer) (bFromSweep :type Boolean) (SweepResult :type Hit%20Result%20Structure%20%28by%20ref%29))
  (bind _asbase_car (Utilities|Casting|CastToBase_Car OtherActor))
  (CallFunction|SetIsBehindTraficLight _asbase_car (Variables|AI|GetIsBehindTrafficLight) (Math|Random|RandomInteger 1000000000)))

(event Custom|Set%20Speed
  (bind _state (Variables|AI|GetState))
  (bind _vehiclemovement (Variables|Default|GetVehicleMovement))
  (bind _returnvalue (Class|WheeledVehicleMovementComponent|GetForwardSpeed _vehiclemovement))
  (bind _returnvalue_2 (* _returnvalue 0.036))
  ;[1 1 1] Cruise Control
  (if (or (Utilities|Enum|Equal(Enum) _state "NewEnumerator5") (Utilities|Enum|Equal(Enum) _state "NewEnumerator6"))
    (Variables|AI|SetTargetSpeed (Variables|AI|GetIdealSpeed))
    (else
      (Variables|AI|SetTargetSpeed (Math|Float|Min(Float) (Variables|AI|GetStreetSpeedLimit) (Variables|AI|GetIdealSpeed)))))
  (if (Utilities|Enum|NotEqual(Enum) _state "NewEnumerator0")
    (if (Math|Float|InRange(Float) _returnvalue_2 (- (Variables|AI|GetTargetSpeed) 1.0) (+ (Variables|AI|GetTargetSpeed) 1.0))
      _
      (else
        (bind _output_get (Variables|AI|SetSpeed (+ (/ (- (Variables|AI|GetTargetSpeed) _returnvalue_2) 3e+02) (Variables|AI|GetSpeed))))
        (Class|WheeledVehicleMovementComponent|SetThrottleInput (Variables|Default|GetVehicleMovement) _output_get)))
    (Utilities|FlowControl|Delay 1.0)
    (CallFunction|SetSpeed)))

(event EventBeginPlay
  (CallFunction|InitializeAIState))

(event EventTick
  (params (DeltaSeconds :type Float%20%28single-precision%29))
  (bind _vehiclemovement (Variables|Default|GetVehicleMovement))
  (bind _paths (Variables|AI|GetPaths))
  (bind _activepathindex (Variables|AI|GetActivePathIndex))
  (bind _output (Utilities|Array|Get(acopy) _paths _activepathindex))
  (Utilities|FlowControl|Sequence
    (:then_0
      ;[1 1 1] AI State Management
      (switch Utilities|FlowControl|Switch|SwitchonAI_State (Variables|AI|GetState)
        (:NewEnumerator3
          (CallFunction|UpdateRandomDriving)
          (if (< (Class|WheeledVehicleMovementComponent|GetForwardSpeed (Variables|Default|GetVehicleMovement)) 5.0)
            (Utilities|FlowControl|DoOnce false :!label _label
              (:Completed
                (Variables|Default|SetIsTimerValid true)
                (Utilities|FlowControl|Delay 1e+01)
                (if (Variables|Default|GetIsTimerValid)
                  (bind _isinview (CallFunction|IsinView :!label _label_2))
                  (if _isinview
                    (Utilities|FlowControl|Delay 0.1)
                    (goto _label_2)
                    (else
                      (Actor|DestroyActor)))
                  (else
                    (goto _label Reset)))))
            (else
              (Variables|Default|SetIsTimerValid false))))
        (:NewEnumerator4
          (CallFunction|UpdateTargetedDriving))
        (:NewEnumerator5
          (CallFunction|UpdateLongChaseDriving))
        (:NewEnumerator6
          (CallFunction|UpdateCloseChaseDriving))))
    (:then_1
      ;[1 1 1] AI Steering input
      (if (Variables|AI|GetIsSteering)
        (if (Variables|AI|GetIsTrackingPath)
          (if (Utilities|IsValid _output)
            (bind _steerning (CallFunction|GetSteeringtoPath _output))
            (Class|WheeledVehicleMovementComponent|SetSteeringInput _vehiclemovement _steerning))
          (else
            (bind _steerning_2 (CallFunction|GetSteeringtoTarget (Variables|AI|GetTarget)))
            (Class|WheeledVehicleMovementComponent|SetSteeringInput _vehiclemovement _steerning_2)))))))

(fn ConstructionScript)

(fn GetSteeringtoPath
  (params (Path :type Spline%20Component%20Object%20Reference))
  (bind _returnvalue (Transformation|GetActorLocation))
  (return (Math|Float|MapRangeClamped (.yaw (Math|Rotator|Delta(Rotator) (Math|Rotator|FindLookatRotation _returnvalue (Spline|FindLocationClosesttoWorldLocation Path (+ (* (Math|Vector|Normalize (Class|SplineComponent|FindTangentClosesttoWorldLocation Path _returnvalue "World")) 5e+02) _returnvalue) "World")) (Transformation|GetActorRotation))) -9e+01 9e+01 -1.0 1.0)))

(fn GetSteeringtoTarget
  (params (Target%20Position :type Vector))
  (return (Math|Float|MapRangeClamped (.yaw (Math|Rotator|Delta(Rotator) (Math|Rotator|FindLookatRotation (Transformation|GetActorLocation) Target%20Position) (Transformation|GetActorRotation))) -9e+01 9e+01 -1.0 1.0)))

(fn GetChaseType
  (return true))

(fn Stop
  (bind _vehiclemovement (Variables|Default|GetVehicleMovement))
  (Class|WheeledVehicleMovementComponent|SetThrottleInput _vehiclemovement 0.0)
  (bind _output_get (Variables|AI|SetIsStanding true))
  (Class|WheeledVehicleMovementComponent|SetHandbrakeInput _vehiclemovement _output_get)
  (Variables|AI|SetSpeed 0.0)
  (Variables|AI|SetIdealSpeed 0.0))

(fn Drive
  (bind _output_get (Variables|AI|SetIsStanding false))
  (Class|WheeledVehicleMovementComponent|SetHandbrakeInput (Variables|Default|GetVehicleMovement) _output_get)
  (CallFunction|SetSpeed))

(fn GotoIdling
  (Variables|AI|SetState "NewEnumerator0")
  (CallFunction|Stop))

(fn GotoRandomDriving
  (params (Paths :type Array%20of%20Spline%20Component%20Object%20References) (ActivePathIndex :type Integer))
  (Variables|AI|SetState "NewEnumerator3")
  (Variables|AI|SetPaths Paths)
  (Variables|AI|SetActivePathIndex ActivePathIndex)
  (Variables|AI|SetIdealSpeed (Variables|AI|GetNormalSpeed))
  (Variables|AI|SetIsTrackingPath true)
  (CallFunction|Drive))

(fn GotoTargetedDriving
  (params (Target :type Vector))
  (Variables|AI|SetState "NewEnumerator4")
  (Variables|AI|SetTarget Target)
  (Variables|AI|SetIdealSpeed (Variables|AI|GetNormalSpeed))
  (Variables|AI|SetIsTrackingPath true)
  (Variables|AI|SetTargetReached false)
  (CallFunction|Drive))

(fn GotoDirectParking
  (params (Target :type Vector))
  (Variables|AI|SetState "NewEnumerator2")
  (Variables|AI|SetTarget Target)
  (Variables|AI|SetIdealSpeed (Variables|AI|GetParkingSpeed))
  (Variables|AI|SetIsTrackingPath false)
  (Variables|AI|SetIsLookingForParkingSpot false)
  (CallFunction|Drive))

(fn GotoGuidedParking
  (params (Paths :type Array%20of%20Spline%20Component%20Object%20References) (ActivatPathIndex :type Integer))
  (Variables|AI|SetState "NewEnumerator1")
  (Variables|AI|SetPaths Paths)
  (Variables|AI|SetActivePathIndex ActivatPathIndex)
  (Variables|AI|SetIdealSpeed (Variables|AI|GetParkingSpeed))
  (Variables|AI|SetIsTrackingPath true)
  (Variables|AI|SetIsLookingForParkingSpot false)
  (CallFunction|Drive))

(fn GotoCloseChaseDriving
  (params (Target :type Vector))
  (Variables|AI|SetState "NewEnumerator6")
  (Variables|AI|SetTarget Target)
  (Variables|AI|SetIdealSpeed (Variables|AI|GetChasingSpeed))
  (Variables|AI|SetIsTrackingPath false)
  (Variables|AI|SetTargetCatched false)
  (CallFunction|Drive))

(fn GotoLongChaseDriving
  (params (Paths :type Array%20of%20Spline%20Component%20Object%20References) (ActivePathIndex :type Integer) (Target :type Vector))
  (Variables|AI|SetState "NewEnumerator6")
  (Variables|AI|SetTarget Target)
  (Variables|AI|SetPaths Paths)
  (Variables|AI|SetActivePathIndex ActivePathIndex)
  (Variables|AI|SetIdealSpeed (Variables|AI|GetChasingSpeed))
  (Variables|AI|SetIsTrackingPath true)
  (Variables|AI|SetTargetCatched false)
  (CallFunction|Drive))

(fn InitializeAIState
  (CallFunction|GotoStatewithPreviousData (Variables|AI|GetState)))

(fn UpdateTargetedDriving
  (if (< (Math|Vector|Distance(Vector) (Variables|AI|GetTarget) (Transformation|GetActorLocation)) (Variables|AI|GetTargetReachRange))
    (Variables|AI|SetTargetReached true)
    (CallFunction|GotoRandomDriving (Variables|AI|GetPaths) (Variables|AI|GetActivePathIndex))))

(fn UpdateRandomDriving
  (if (== (Math|Random|RandomInteger 10000) 0)
    (Variables|AI|SetIsLookingForParkingSpot true)))

(fn UpdateLongChaseDriving
  (bind _targetcar (Variables|AI|GetTargetCar))
  (Variables|AI|SetTarget (Transformation|GetActorLocation _targetcar))
  (if (> (Math|Vector|Distance(Vector) (Variables|AI|GetTarget) (Transformation|GetActorLocation)) (Variables|AI|GetChasingRange))
    (CallFunction|GotoRandomDriving (Variables|AI|GetPaths) (Variables|AI|GetActivePathIndex))
    (elif (== (Variables|AI|GetStreetGUID) (Variables|Base_Car_C|GetStreetGUID _targetcar))
      (CallFunction|GotoCloseChaseDriving (Variables|AI|GetTarget)))))

(fn UpdateCloseChaseDriving
  (bind _targetcar (Variables|AI|GetTargetCar))
  (Variables|AI|SetTarget (Transformation|GetActorLocation _targetcar))
  (if (or (> (Math|Vector|Distance(Vector) (Variables|AI|GetTarget) (Transformation|GetActorLocation)) (Variables|AI|GetChasingRange)) (!= (Variables|AI|GetStreetGUID) (Variables|Base_Car_C|GetStreetGUID _targetcar)))
    (CallFunction|GotoLongChaseDriving (Variables|AI|GetPaths) (Variables|AI|GetActivePathIndex) (Variables|AI|GetTarget))
    (elif (< (Math|Vector|Distance(Vector) (Variables|AI|GetTarget) (Transformation|GetActorLocation)) (Variables|AI|GetCatchRange))
      (Variables|AI|SetTargetCatched true))))

(fn GotoStatewithPreviousData
  (params (State :type AI_State%20Enum :default "NewEnumerator0"))
  (bind _paths (Variables|AI|GetPaths))
  (bind _activepathindex (Variables|AI|GetActivePathIndex))
  (bind _target (Variables|AI|GetTarget))
  (switch Utilities|FlowControl|Switch|SwitchonAI_State State
    (:NewEnumerator0
      (CallFunction|GotoIdling))
    (:NewEnumerator1
      (CallFunction|GotoGuidedParking _paths _activepathindex))
    (:NewEnumerator2
      (CallFunction|GotoDirectParking _target))
    (:NewEnumerator3
      (CallFunction|GotoRandomDriving _paths _activepathindex))
    (:NewEnumerator4
      (CallFunction|GotoTargetedDriving _target))
    (:NewEnumerator5
      (CallFunction|GotoLongChaseDriving _paths _activepathindex _target))
    (:NewEnumerator6
      (CallFunction|GotoCloseChaseDriving _target))))

(fn SetIsBehindTraficLight
  (params (value :type Boolean) (ChainId :type Integer))
  (if (not (== ChainId (Variables|Default|GetLastChainId)))
    (bind _output_get (Variables|Default|SetLastChainId ChainId))
    (bind _output_get_2 (Variables|AI|SetIsBehindTrafficLight value))
    (for _array_element (Collision|GetOverlappingActors (Variables|Default|GetRed%20Light%20Zone) "Base_Car_C" :!class /Script/Engine.PrimitiveComponent)
      (bind _asbase_car (Utilities|Casting|CastToBase_Car _array_element))
      (CallFunction|SetIsBehindTraficLight _asbase_car _output_get_2 _output_get))))

(fn IsinView
  (bind _returnvalue (Game|GetPlayerController 0))
  (bind _returnvalue_2 (Transformation|GetActorLocation))
  (bind _returnvalue_3 (Viewport|GetViewportSize))
  (bind _returnvalue_4 (Utilities|IsValid _returnvalue))
  (bind _screenlocation (Class|PlayerController|ProjectWorldLocationtoScreen _returnvalue _returnvalue_2 false))
  (return (or (Math|Boolean|ANDBoolean (> (.y _screenlocation) 0.0) (> (.x _screenlocation) 0.0) (< (.x _screenlocation) (.x _returnvalue_3)) (< (.y _screenlocation) (.y _returnvalue_3)) _returnvalue_4) (not _returnvalue_4))))