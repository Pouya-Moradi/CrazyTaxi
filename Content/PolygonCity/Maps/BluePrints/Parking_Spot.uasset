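; Parking spot actor that lets AI Base_Car vehicles pull in, idle for a short random time and drive out.
; A start trigger claims the free spot for a car looking for parking, saves its route and sends it along the guided Spline.
; The spot trigger idles that car, then resumes the Spline.
; The end trigger frees the spot and returns the car to random driving on its saved route.
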(event OnComponentBeginOverlap(StartParkingTrigger)
  (params (OverlappedComponent :type Primitive%20Component%20Object%20Reference) (OtherActor :type Actor%20Object%20Reference) (OtherComp :type Primitive%20Component%20Object%20Reference) (OtherBodyIndex :type Integer) (bFromSweep :type Boolean) (SweepResult :type Hit%20Result%20Structure%20%28by%20ref%29))
  (bind _asbase_car (Utilities|Casting|CastToBase_Car OtherActor))
  (if (not (Variables|Default|GetIsFull))
    (if (Variables|/Game/PolygonCity/Maps/BluePrints/Base_Car_BP/Base_Car.Base_Car_C|GetIsLookingForParkingSpot _asbase_car)
      (Variables|Default|SetParkedCarPaths (Variables|/Game/PolygonCity/Maps/BluePrints/Base_Car_BP/Base_Car.Base_Car_C|GetPaths _asbase_car))
      (Variables|Default|SetParkedCarActivePathIndex (Variables|/Game/PolygonCity/Maps/BluePrints/Base_Car_BP/Base_Car.Base_Car_C|GetActivePathIndex _asbase_car))
      (Variables|Default|SetIsFull true)
      (Variables|Default|SetParkedCar _asbase_car)
      (Default|GotoGuidedParking _asbase_car (Utilities|Array|MakeArray (Variables|Default|GetSpline))))))

(event OnComponentBeginOverlap(ParkingSpot)
  (params (OverlappedComponent :type Primitive%20Component%20Object%20Reference) (OtherActor :type Actor%20Object%20Reference) (OtherComp :type Primitive%20Component%20Object%20Reference) (OtherBodyIndex :type Integer) (bFromSweep :type Boolean) (SweepResult :type Hit%20Result%20Structure%20%28by%20ref%29))
  (bind _asbase_car (Utilities|Casting|CastToBase_Car OtherActor))
  (if (== _asbase_car (Variables|Default|GetParkedCar))
    (Default|GotoIdling _asbase_car)
    (Utilities|FlowControl|RetriggerableDelay (Math|Random|RandomFloatinRange 5.0 1e+01))
    (Default|GotoGuidedParking _asbase_car (Utilities|Array|MakeArray (Variables|Default|GetSpline)))))

(event OnComponentBeginOverlap(EndParkingTrigger)
  (params (OverlappedComponent :type Primitive%20Component%20Object%20Reference) (OtherActor :type Actor%20Object%20Reference) (OtherComp :type Primitive%20Component%20Object%20Reference) (OtherBodyIndex :type Integer) (bFromSweep :type Boolean) (SweepResult :type Hit%20Result%20Structure%20%28by%20ref%29))
  (bind _asbase_car (Utilities|Casting|CastToBase_Car OtherActor))
  (if (== _asbase_car (Variables|Default|GetParkedCar))
    (Variables|Default|SetIsFull false)
    (Default|GotoRandomDriving _asbase_car (Variables|Default|GetParkedCarPaths) (Variables|Default|GetParkedCarActivePathIndex))))

(fn ConstructionScript)